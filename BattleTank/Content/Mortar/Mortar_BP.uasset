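; Mortar Blueprint for a weapon emplacement built from body, dome and barrel static meshes.
; The construction script assigns the meshes and sets the aiming component's projectile class to Projetile_BP.
; On BeginPlay it initialises the TankAiming component with the dome as turret and the barrel as barrel, reusing tank aiming for the mortar.
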(event `self.ReceiveBeginPlay`
  (`TankAimingComponent.Initialise` (`self.TankAiming`) (`self.MortarDome`) (`self.MortarBarrel`)))

(fn `UserConstructionScript`
  (`StaticMeshComponent.SetStaticMesh` (`self.MortarBody`) "/Game/Mortar/mortar_body.mortar_body")
  (`StaticMeshComponent.SetStaticMesh` (`self.MortarDome`) "/Game/Mortar/mortar_dome.mortar_dome")
  (`StaticMeshComponent.SetStaticMesh` (`self.MortarBarrel`) "/Game/Mortar/mortar_barrel.mortar_barrel")
  (set `TankAimingComponent.ProjectileBP` "/Game/Tank/Projetile_BP.Projetile_BP_C" (`self.TankAiming`)))