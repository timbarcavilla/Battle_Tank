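; Player controller Blueprint for the tank player that creates and manages the HUD and end-of-game screens.
; When a tank is found, it creates the player UI widget and passes it the controller, tank and aiming component references.
; Death and victory events show their menus with the mouse cursor, while a level increase removes all widgets.
; The construction script sets the tank class to Tank_BP.
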(event `self.FoundTank`
  (params (TankRef :type "Tank Object Reference"))
  (bind _returnvalue (`|CreateWidget` "/Game/PlayerUI.PlayerUI_C"))
  (set `/Game/PlayerUI.PPController` self _returnvalue)
  (set `/Game/PlayerUI.TankRef` TankRef _returnvalue)
  (set `/Game/PlayerUI.BP Aim Comp Ref` (`self.GetComponentByClass` TankRef "/Script/BattleTank.TankAimingComponent") _returnvalue)
  (`UserWidget.AddToViewport` _returnvalue 0))

(event `self.DisplayDeathMenu`
  (bind _returnvalue (`|CreateWidget` "/Game/Blueprints/DeathScreen_BP.DeathScreen_BP_C"))
  (`UserWidget.AddToViewport` _returnvalue 0)
  (`Widget.SetVisibility` _returnvalue "Visible")
  (set `self.bShowMouseCursor` true))

(event `self.DisplayVictoryMenu`
  (bind _returnvalue (`|CreateWidget` "/Game/Blueprints/VictoryScreen_BP.VictoryScreen_BP_C"))
  (`UserWidget.AddToViewport` _returnvalue 0)
  (`Widget.SetVisibility` _returnvalue "Visible")
  (set `/Game/Blueprints/VictoryScreen_BP.PPController` self _returnvalue)
  (set `self.bShowMouseCursor` true))

(event `self.LevelIncreased`
  (`WidgetLayoutLibrary.RemoveAllWidgets`))

(fn `UserConstructionScript`
  (set `self.TankBP` "/Game/Tank/Tank_BP.Tank_BP_C"))